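; Spell entity movement component that adds a parabolic arc by pulling LinearVelocity down by Gravity each tick, after the parent tick.
; ComputeMaxDistance derives flat-ground range from squared speed over gravity.
; A helper turns a desired distance into a low-arc launch pitch via arcsine, warning and using 45 degrees when unreachable.
; It returns a pitched forward vector scaled by that maximum distance, not by speed.
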(event EventBeginPlay
  (|CallParentFunction) ; This node is disabled and will not be called.\nDrag off pins to build functionality.
)

(event EventTick
  (params (DeltaSeconds :type Float%20%28single-precision%29))
  (|CallParentFunction DeltaSeconds)
  (Variables|Default|SetlinearVelocity (+ (Variables|Default|GetlinearVelocity) (* (Math|Vector|VectorDown) (Variables|Default|GetGravity) DeltaSeconds))))

(fn ComputeMaxDistance
  (bind _linearvelocity (Variables|Default|GetlinearVelocity))
  (return (/ (Math|Vector|DotProduct _linearvelocity _linearvelocity) (Variables|Default|GetGravity))))

(fn ComputeVelocitywithDesiredDistancewithAngle
  (params (DesiredDistance :type Float%20%28double-precision%29))
  (LocalVariables|SetMaxDistance (CallFunction|ComputeMaxDistance))
  (if (<= (/ DesiredDistance (LocalVariables|GetMaxDistance)) 1.0)
    (LocalVariables|Setangle_deg (* (Class|KismetMathLibrary|DegAsin (/ DesiredDistance (LocalVariables|GetMaxDistance))) 0.5))
    (else
      (Development|PrintString "Warning: Desired distance is impossible")
      (LocalVariables|Setangle_deg 45.0)))
  (return (Math|Vector|RotateVector (* (Class|KismetMathLibrary|VectorForward) (LocalVariables|GetMaxDistance)) (Math|Rotator|MakeRotator 0.0 (LocalVariables|Getangle_deg) 0.0))))