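; Base character Blueprint that sets up Enhanced Input for spell casting, with placeholder actions only.
; On BeginPlay it adds the spell mapping context to the controlling player's Enhanced Input subsystem through a helper that reports success or an invalid subsystem.
; Fire, Life, Earth and Water spell input actions each just print debug text, with Fire handling both Started and Triggered.
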(event EventBeginPlay
  (CallFunction|MapInputMappingContext "/Game/Inputs/IMC_Spell.IMC_Spell"))

(event Input|EnhancedActionEvents|EnhancedInputActionIA_SpellFire
  (params (ActionValue :type Boolean) (ElapsedSeconds :type Float%20%28double-precision%29) (TriggeredSeconds :type Float%20%28double-precision%29) (InputAction :type Input%20Action%20Object%20Reference :default "/Game/Inputs/InputAction/IA_SpellFire.IA_SpellFire"))
  (:Triggered
    (Development|PrintString "Hello"))
  (:Started
    (Development|PrintString "Start")))

(event Input|EnhancedActionEvents|EnhancedInputActionIA_SpellLife
  (params (ActionValue :type Boolean) (ElapsedSeconds :type Float%20%28double-precision%29) (TriggeredSeconds :type Float%20%28double-precision%29) (InputAction :type Input%20Action%20Object%20Reference :default "/Game/Inputs/InputAction/IA_SpellLife.IA_SpellLife"))
  (Development|PrintString "Life"))

(event Input|EnhancedActionEvents|EnhancedInputActionIA_Spell_Earth
  (params (ActionValue :type Boolean) (ElapsedSeconds :type Float%20%28double-precision%29) (TriggeredSeconds :type Float%20%28double-precision%29) (InputAction :type Input%20Action%20Object%20Reference :default "/Game/Inputs/InputAction/IA_Spell_Earth.IA_Spell_Earth"))
  (Development|PrintString "Earth"))

(event Input|EnhancedActionEvents|EnhancedInputActionIA_SpellWater
  (params (ActionValue :type Boolean) (ElapsedSeconds :type Float%20%28double-precision%29) (TriggeredSeconds :type Float%20%28double-precision%29) (InputAction :type Input%20Action%20Object%20Reference :default "/Game/Inputs/InputAction/IA_SpellWater.IA_SpellWater"))
  (Development|PrintString "Water"))

(fn ConstructionScript)

(fn MapInputMappingContext
  (params (MappingContext :type Input%20Mapping%20Context%20Object%20Reference))
  (bind _asplayer_controller (Utilities|Casting|CastToPlayerController (Pawn|GetController)))
  (Utilities|IsValid (PlayerController|LocalPlayerSubsystems|GetEnhancedInputLocalPlayerSubsystem _asplayer_controller)
    (:Is%20Valid
      (Input|AddMappingContext (PlayerController|LocalPlayerSubsystems|GetEnhancedInputLocalPlayerSubsystem _asplayer_controller) MappingContext 0 "(bIgnoreAllPressedKeysUntilRelease=True,bForceImmediately=False,bNotifyUserSettings=False)")
      (Development|PrintString "Mapped"))
    (:Is%20Not%20Valid
      (Development|PrintString "Error: Input Local Subsystem is invalid"))))